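; BP_ColorSphere is a collectible that changes the overlapping character's outline color or, as a checkpoint, sets its respawn point and active part.
; Checkpoints also destroy or reveal tagged level actors.
; Timelines animate spawning, idle motion and collection, while Tick counts down to respawn unless the sphere is destroyed as single-use.
; The construction script stores the spawn location and drives color and pulse through a dynamic material, also tinting the dust particles.
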(event Custom|Spawn
  ;[1 1 1] Spawn
  (Variables|Default|SetbIsCollected false)
  (bind (_direction _locationz _uniformscale) (Timeline|SpawnTimeline PlayFromStart)
    (:Update
      (Transformation|SetActorLocation (+ (* (Transformation|GetActorUpVector) _locationz) (Variables|Spawn|GetSpawnLocation)) false)
      (Transformation|SetActorScale3D (Math|Vector|MakeVector _uniformscale _uniformscale _uniformscale)))
    (:Finished
      (CallFunction|Idle))))

(event Custom|Idle
  ;[1 1 1] Idle Animation
  (bind _locationz (Timeline|IdleTimeline PlayFromStart)
    (:Update
      (Transformation|SetActorLocation (+ (Variables|Spawn|GetSpawnLocation) (* (Transformation|GetActorUpVector) _locationz)) false))))

(event EventActorBeginOverlap
  (params (OtherActor :type Actor%20Object%20Reference))
  (bind _returnvalue (Transformation|GetActorLocation))
  ;[1 1 1] OnCollect
  (Utilities|FlowControl|Sequence
    (:then_0
      (bind _asbp_character (Utilities|Casting|CastToBP_Character OtherActor))
      (if (Variables|Default|GetbIsCheckpoint)
        (Variables|/Game/Blueprints/BP_Character.BP_Character_C|SetActiveTag _asbp_character (Variables|Default|GetActivePart))
        (Variables|/Game/Blueprints/BP_Character.BP_Character_C|SetRespawnPoint _asbp_character (Transformation|GetActorLocation))
        (bind _outactors (Actor|GetAllActorsOfClass "/Script/Engine.Actor"))
        (for _array_element _outactors
          (if (Actor|ActorHasTag _array_element (Variables|Default|GetRemovePreviousPart))
            (Actor|DestroyActor _array_element)
            (elif (Actor|ActorHasTag _array_element (Variables|Default|GetShowNextPart))
              (bind _asbp_colored_platform (Utilities|Casting|CastToBP_ColoredPlatform _array_element)
                (:then
                  (Default|SetVisibility _asbp_colored_platform true))
                (:CastFailed
                  (Rendering|SetActorHiddenInGame _array_element false))))))
        (else
          (Default|ChangeOutlineColor _asbp_character (Variables|Color|GetOutlineColor)))))
    (:then_2
      (if (not (Variables|Default|GetbIsCollected))
        (Audio|Components|Audio|Stop)
        (Audio|Components|Audio|Stop)
        (bind _asbp_game_instance (Utilities|Casting|CastToBP_GameInstance (Game|GetGameInstance))
          (:then
            _)
          (:CastFailed
            _))
        (Audio|PlaySoundatLocation "/Game/SoundEffects/swoop02.swoop02" _returnvalue (Variables|/Game/Blueprints/BP_GameInstance.BP_GameInstance_C|GetMasterVolume _asbp_game_instance))
        (Variables|Default|SetbIsCollected true)
        (bind _returnvalue_2 (Effects|SpawnEmitteratLocation "/Game/ParticleEffects/P_CollectSphere.P_CollectSphere" _returnvalue))
        (Effects|Components|ParticleSystem|SetColorParameter _returnvalue_2 "ParticleColor" (Variables|Color|GetOutlineColor))
        (bind _uniformscale (Timeline|CollectTimeline Play)
          (:Update
            (Transformation|SetActorScale3D (Math|Vector|MakeVector _uniformscale _uniformscale _uniformscale)))
          (:Finished
            (if (Variables|Default|GetbSpawnOnlyOnce)
              (Actor|DestroyActor))))))))

(event EventTick
  (params (DeltaSeconds :type Float%20%28single-precision%29))
  (Variables|Default|SetDeltaTime DeltaSeconds)
  (Utilities|FlowControl|Sequence
    (:then_0
      ;[1 1 1] Respawn Timer
      (if (Variables|Default|GetbIsCollected)
        (Variables|Spawn|SetRespawnTimer (+ (Variables|Spawn|GetRespawnTimer) (Variables|Default|GetDeltaTime)))
        (if (>= (Variables|Spawn|GetRespawnTimer) (Variables|Spawn|GetRespawnTime))
          (Variables|Spawn|SetRespawnTimer 0.0)
          (CallFunction|Spawn))))))

(event EventBeginPlay
  ;[1 1 1] Begin Play
  (Utilities|FlowControl|Delay (Variables|Default|GetInitialSpawnDelay))
  (CallFunction|Spawn))

(fn ConstructionScript
  (bind _returnvalue (Rendering|Material|CreateDynamicMaterialInstance (Variables|Default|GetSphere) 0 "/Game/Materials/Mat_ColorWithOutline.Mat_ColorWithOutline" :!class /Script/Engine.PrimitiveComponent))
  (Variables|Color|SetMID _returnvalue)
  (Utilities|FlowControl|Sequence
    (:then_0
      (Rendering|Material|SetVectorParameterValue (Variables|Color|GetMID) "BaseColorTint" (Variables|Color|GetBaseColor) :!class /Script/Engine.MaterialInstanceDynamic))
    (:then_1
      (Rendering|Material|SetVectorParameterValue (Variables|Color|GetMID) "OutlineColor" (Variables|Color|GetOutlineColor) :!class /Script/Engine.MaterialInstanceDynamic))
    (:then_2
      (Rendering|Material|SetScalarParameterValue (Variables|Color|GetMID) "EnablePulse" (Math|Float|SelectFloat 0.0 1.0 (Variables|Color|GetbIsPulsing)) :!class /Script/Engine.MaterialInstanceDynamic))
    (:then_3
      (Rendering|Material|SetScalarParameterValue (Variables|Color|GetMID) "PulseDuration" (Variables|Color|GetPulseDuration) :!class /Script/Engine.MaterialInstanceDynamic))
    (:then_4
      (Rendering|Material|SetScalarParameterValue (Variables|Color|GetMID) "PulseIntensity" (Variables|Color|GetOutlineIntensity) :!class /Script/Engine.MaterialInstanceDynamic))
    (:then_5
      (Variables|Spawn|SetSpawnLocation (Transformation|GetActorLocation)))
    (:then_6
      (Effects|Components|ParticleSystem|SetColorParameter (Variables|Default|GetDust) "ParticleColor" (Variables|Color|GetOutlineColor)))))