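; BP_Tutorial is a one-shot overlap trigger that shows a four-line tutorial widget to the BP_Character.
; On overlap it removes the display of its linked PreviousTutorial, then creates UMG_Tutorial with its own lines and adds it to the viewport.
; Tick then counts up to MaxTimeAlive, removes the widget and destroys the actor.
; The triggered flag is set before the character cast, so any overlapping actor uses up the trigger.
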(event EventActorBeginOverlap
  (params (OtherActor :type Actor%20Object%20Reference))
  (bind _previoustutorial (Variables|Default|GetPreviousTutorial))
  (if (not (Variables|Default|GetbWasTriggered))
    (Variables|Default|SetbWasTriggered true)
    (Utilities|Casting|CastToBP_Character OtherActor)
    (Utilities|IsValid _previoustutorial
      (:Is%20Valid
        (Widget|RemovefromParent (Variables|BP_Tutorial_C|GetTutorialDisplay _previoustutorial)))
      (:Is%20Not%20Valid
        _))
    (bind _returnvalue (UserInterface|CreateWidget "/Game/Blueprints/UI/UMG_Tutorial.UMG_Tutorial_C" 0 (Variables|Default|GetLine01) (Variables|Default|GetLine02) (Variables|Default|GetLine03) (Variables|Default|GetLine04)))
    (Variables|Default|SetTutorialDisplay _returnvalue)
    (UserInterface|Viewport|AddtoViewport _returnvalue)))

(event EventTick
  (params (DeltaSeconds :type Float%20%28single-precision%29))
  (Variables|Default|SetDeltaTIme DeltaSeconds)
  (if (Variables|Default|GetbWasTriggered)
    (Variables|Default|SetAliveTimer (+ (Variables|Default|GetAliveTimer) (Variables|Default|GetDeltaTIme)))
    (if (>= (Variables|Default|GetAliveTimer) (Variables|Default|GetMaxTimeAlive))
      (Widget|RemovefromParent (Variables|Default|GetTutorialDisplay))
      (Actor|DestroyActor))))

(fn ConstructionScript)