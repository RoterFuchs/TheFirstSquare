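; BP_FirstSquare is a one-time collectible that launches the player skyward and triggers a cinematic leading to the credits.
; On first overlap it plays a sound and tinted burst, then launches BP_Character.
; If its Matinee is valid, it plays it, animates its scale by timeline and, five seconds later, shows HUD credits and moves the player to the origin.
; The construction script sets dynamic-material colors and pulse, and tints the dust.
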(event EventActorBeginOverlap
  (params (OtherActor :type Actor%20Object%20Reference))
  (bind _returnvalue (Transformation|GetActorLocation))
  (bind _matinee (Variables|Default|GetMatinee))
  ;[1 1 1] OnCollect
  (Utilities|FlowControl|Sequence
    (:then_2
      (if (not (Variables|Default|GetbIsCollected))
        (Audio|PlaySoundatLocation "/Game/SoundEffects/swoop02.swoop02" _returnvalue)
        (Variables|Default|SetbIsCollected true)
        (bind _returnvalue_2 (Effects|SpawnEmitteratLocation "/Game/ParticleEffects/P_CollectSphere.P_CollectSphere" _returnvalue))
        (Effects|Components|ParticleSystem|SetColorParameter _returnvalue_2 "ParticleColor" (Variables|Color|GetOutlineColor))
        (bind _asbp_character (Utilities|Casting|CastToBP_Character OtherActor))
        (Character|LaunchCharacter _asbp_character "0, 0,50000.000000" false true)
        (Utilities|IsValid _matinee
          (:Is%20Valid
            (Audio|Components|Audio|Play _matinee)
            (Utilities|FlowControl|Sequence
              (:then_0
                (bind _uniformscale (Timeline|CollectTimeline PlayFromStart)
                  (:Update
                    (Transformation|SetActorScale3D (Math|Vector|MakeVector _uniformscale _uniformscale _uniformscale)))))
              (:then_1
                (Utilities|FlowControl|Delay 5.0)
                (bind _asbp_hud (Utilities|Casting|CastToBP_HUD (HUD|GetHUD (Game|GetPlayerController 0))))
                (Default|ShowCredits _asbp_hud)
                (Transformation|SetActorLocation (Game|GetPlayerCharacter 0) "0, 0, 0" false)))))))))

(fn ConstructionScript
  (bind _returnvalue (Rendering|Material|CreateDynamicMaterialInstance (Variables|Default|GetSphere) 0 "/Game/Materials/Mat_ColorWithOutline_RandomColor.Mat_ColorWithOutline_RandomColor" :!class /Script/Engine.PrimitiveComponent))
  (Variables|Color|SetMID _returnvalue)
  (Utilities|FlowControl|Sequence
    (:then_0
      (Rendering|Material|SetVectorParameterValue (Variables|Color|GetMID) "BaseColorTint" (Variables|Color|GetBaseColor) :!class /Script/Engine.MaterialInstanceDynamic))
    (:then_1
      (Rendering|Material|SetVectorParameterValue (Variables|Color|GetMID) "OutlineColor" (Variables|Color|GetOutlineColor) :!class /Script/Engine.MaterialInstanceDynamic))
    (:then_2
      (Rendering|Material|SetScalarParameterValue (Variables|Color|GetMID) "EnablePulse" (Math|Float|SelectFloat 0.0 1.0 (Variables|Color|GetbIsPulsing)) :!class /Script/Engine.MaterialInstanceDynamic))
    (:then_3
      (Rendering|Material|SetScalarParameterValue (Variables|Color|GetMID) "PulseDuration" (Variables|Color|GetPulseDuration) :!class /Script/Engine.MaterialInstanceDynamic))
    (:then_4
      (Rendering|Material|SetScalarParameterValue (Variables|Color|GetMID) "PulseIntensity" (Variables|Color|GetOutlineIntensity) :!class /Script/Engine.MaterialInstanceDynamic))
    (:then_5
      (Variables|Spawn|SetSpawnLocation (Transformation|GetActorLocation)))
    (:then_6
      (Effects|Components|ParticleSystem|SetColorParameter (Variables|Default|GetDust) "ParticleColor" (Variables|Color|GetOutlineColor)))))