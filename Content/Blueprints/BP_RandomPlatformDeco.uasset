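; Decoration Blueprint that scatters randomly transformed mesh instances, by its name platform dressing, when the construction script runs.
; The construction script loops over Amount, adding an instance with random location, rotation and scale from three helper functions.
; Each helper draws per axis from its own random stream, keeping layouts repeatable for a given seed.
; Z scale allows ten times the maximum, so pieces can stretch tall along their local axis.
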(fn ConstructionScript
  (for _index (range 0 (Variables|Default|GetAmount))
    (bind _location (CallFunction|GetRandomLocation))
    (bind _rotation (CallFunction|GetRandomRotation))
    (bind _scale (CallFunction|GetRandomScale))
    (Components|InstancedStaticMesh|AddInstance (Math|Transform|MakeTransform _location _rotation _scale))))

(fn GetRandomLocation
  (return (Math|Vector|MakeVector (Math|Random|RandomFloatinRangefromStream (Variables|Default|GetMinDistance) (Variables|Default|GetMaxDistance) (Variables|Default|GetLocationRandomStream)) (Math|Random|RandomFloatinRangefromStream (Variables|Default|GetMinDistance) (Variables|Default|GetMaxDistance) (Variables|Default|GetLocationRandomStream)) (Math|Random|RandomFloatinRangefromStream (Variables|Default|GetMinDistance) (Variables|Default|GetMaxDistance) (Variables|Default|GetLocationRandomStream)))))

(fn GetRandomRotation
  (return (Class|KismetMathLibrary|MakeRot (Math|Random|RandomFloatinRangefromStream 0.0 3.6e+02 (Variables|Default|GetRotationRandomStream)) (Math|Random|RandomFloatinRangefromStream 0.0 3.6e+02 (Variables|Default|GetRotationRandomStream)) (Math|Random|RandomFloatinRangefromStream 0.0 3.6e+02 (Variables|Default|GetRotationRandomStream)))))

(fn GetRandomScale
  (return (Math|Vector|MakeVector (Math|Random|RandomFloatinRangefromStream (Variables|Default|GetMinScale) (Variables|Default|GetMaxScale) (Variables|Default|GetScaleRandomStream)) (Math|Random|RandomFloatinRangefromStream (Variables|Default|GetMinScale) (Variables|Default|GetMaxScale) (Variables|Default|GetScaleRandomStream)) (Math|Random|RandomFloatinRangefromStream (Variables|Default|GetMinScale) (* (Variables|Default|GetMaxScale) 1e+01) (Variables|Default|GetScaleRandomStream)))))