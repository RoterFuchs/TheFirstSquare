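; BP_Lift is an actor that pushes the player character along the lift's up vector while it stands inside a Box trigger.
; Box overlap begin stores the overlapping BP_Character and overlap end clears it when that same actor leaves.
; Tick applies a force scaled by LiftForce to the stored character every frame, tracking only one character at a time.
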(event OnComponentBeginOverlap(Box)
  (params (OtherActor :type Actor%20Object%20Reference) (OtherComp :type Primitive%20Component%20Object%20Reference) (OtherBodyIndex :type Integer) (bFromSweep :type Boolean) (SweepResult :type Hit%20Result%20Structure%20%28by%20ref%29))
  (bind _asbp_character (Utilities|Casting|CastToBP_Character OtherActor))
  (Variables|Default|SetCharacter _asbp_character))

(event OnComponentEndOverlap(Box)
  (params (OtherActor :type Actor%20Object%20Reference) (OtherComp :type Primitive%20Component%20Object%20Reference) (OtherBodyIndex :type Integer))
  (if (== OtherActor (Variables|Default|GetCharacter))
    (Variables|Default|SetCharacter 0)))

(event EventTick
  (params (DeltaSeconds :type Float%20%28single-precision%29))
  (bind _character (Variables|Default|GetCharacter))
  (Variables|Default|SetDeltaTime DeltaSeconds)
  (Utilities|IsValid _character
    (:Is%20Valid
      (Physics|AddForce _character (* (Transformation|GetActorUpVector) (* 1.0 (Variables|Default|GetLiftForce)))))))

(fn ConstructionScript)