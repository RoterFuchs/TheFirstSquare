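; BP_ColoredPlatform is a tinted platform actor that can be shown or hidden along with its collision.
; The construction script creates a dynamic instance of Mat_PlainColor on the mesh, tints it with BaseColor, and applies the initial IsVisible state.
; The SetVisibility event stores a new IsVisible value and toggles both hidden-in-game and collision, so a hidden platform is also non-solid.
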(event Custom|SetVisibility
  (params (bIsVisible :type Boolean))
  (bind _mesh (Variables|Default|GetMesh))
  ;[1 1 1] Toggle Actor Visibility
  (Variables|Default|SetbIsVisible bIsVisible)
  (if bIsVisible
    (Rendering|SetActorHiddenInGame false)
    (Collision|SetCollisionEnabled _mesh "QueryAndPhysics")
    (else
      (Rendering|SetActorHiddenInGame true)
      (Collision|SetCollisionEnabled _mesh "NoCollision"))))

(fn ConstructionScript
  (Utilities|FlowControl|Sequence
    (:then_0
      (bind _returnvalue (Rendering|Material|CreateDynamicMaterialInstance (Variables|Default|GetMesh) 0 "/Game/Materials/Mat_PlainColor.Mat_PlainColor" :!class /Script/Engine.PrimitiveComponent))
      (Variables|Default|SetMID _returnvalue)
      (Rendering|Material|SetVectorParameterValue _returnvalue "BaseColorTint" (Variables|Default|GetBaseColor) :!class /Script/Engine.MaterialInstanceDynamic))
    (:then_1
      (if (Variables|Default|GetbIsVisible)
        (Rendering|SetActorHiddenInGame false)
        (Collision|SetCollisionEnabled "QueryAndPhysics")
        (else
          (Rendering|SetActorHiddenInGame true)
          (Collision|SetCollisionEnabled "NoCollision"))))))